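; BP_Hello is an overlap-triggered actor that plays a greeting and an answering greeting, apparently for a waiting room.
; Any overlapping actor triggers a random HalloSingle sound at its own location.
; After a short random delay, a random HelloBack sound replies from WartezimmerLocation with randomized pitch.
; Both sounds share the waiting room attenuation, and the overlap has no actor filter.
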(event `self.ReceiveActorBeginOverlap`
  (params (OtherActor :type "Actor Object Reference"))
  (bind (_returnvalue_location _returnvalue_rotation) (`KismetMathLibrary.BreakTransform` (`self.GetTransform` OtherActor)))
  (`GameplayStatics.PlaySoundAtLocation` (`KismetArrayLibrary.Array_Random` (`self.HalloSingle`)) _returnvalue_location _returnvalue_rotation 1.0 1.0 0.0 "/Game/Photosynthese/Audio/Praxis/AttentSpat/SA_WaintingRoom.SA_WaintingRoom" null null null)
  (`KismetSystemLibrary.Delay` (`KismetMathLibrary.RandomFloatInRange` 0.5 1.3))
  (`GameplayStatics.PlaySoundAtLocation` (`KismetArrayLibrary.Array_Random` (`self.HelloBack`)) (`self.WartezimmerLocation`) (struct) 1.0 (`KismetMathLibrary.RandomFloatInRange` 1.0 1.3) 0.0 "/Game/Photosynthese/Audio/Praxis/AttentSpat/SA_WaintingRoom.SA_WaintingRoom" null null null))

(fn `UserConstructionScript`)