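; Interactive dream image actor that sends the player into another level once dreamed on long enough.
; Repeated Dream calls increment a counter while a one-shot timeline raises the mesh and boosts its emissive Power through a dynamic material.
; At the DreamStart count, DreamIn animates the pixel-sort parameter collection's Alpha, then opens TestLevel_BigOne.
; InterruptedDream clears the counter, re-arms the DoOnce and reverses the glow and lift.
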(event `self.ReceiveBeginPlay`
  (bind _returnvalue (`PrimitiveComponent.CreateDynamicMaterialInstance` (`self.Interact`) 0 "/Game/Photosynthese/Materials/Emissives/M_EmissiveRed0.M_EmissiveRed0" "None"))
  (set `self.InteractMat` _returnvalue))

(event `self.ReceiveTick`
  (params (DeltaSeconds :type "Float (single-precision)")))

(event `DreamIn`
  (bind (_direction _newtrack_0) (`Timeline|Timeline`)
    (:`Update`
      (`KismetMaterialLibrary.SetScalarParameterValue` "/Game/Photosynthese/Gameplay/DreamLevel/Transitions/PC_PixelSort.PC_PixelSort" "Alpha" _newtrack_0))
    (:`Finished`
      (`GameplayStatics.OpenLevelBySoftObjectPtr` "/Game/Level1/Maps/TestLevel_BigOne.TestLevel_BigOne"))))

(event `self.Dream`
  (bind _result (`/Engine/EditorBlueprintResources/StandardMacros.IncrementInt` (`self.Counter`))
    (:`  `
      (bind _output_get (set `self.Counter` _result))
      (if (== _output_get (`self.DreamStart`))
        (set `self.Counter` 0)
        (`self.DreamIn`)
        (else
          (`/Engine/EditorBlueprintResources/StandardMacros.DoOnce` false :!label _label
            (:`Completed`
              (bind (_direction _newtrack_0) (`Timeline|Timeline_0` :!label _label_2)
                (:`Update`
                  (`MaterialInstanceDynamic.SetScalarParameterValue` (`self.InteractMat`) "Power" (* _newtrack_0 10.0))
                  (`SceneComponent.K2_SetRelativeLocation` (`self.StaticMesh`) (`KismetMathLibrary.MakeVector` 0.0 0.0 (`KismetMathLibrary.Lerp` 0.0 30.0 _newtrack_0)) false false))))))))))

(event `self.InterruptedDream`
  (set `self.Counter` 0)
  (`|ExecutionSequence`
    (:`then_0`
      (goto _label :!via `Reset`))
    (:`then_1`
      (goto _label_2 :!via `Stop`))
    (:`then_2`
      (goto _label_2 :!via `Reverse`))))

(fn `UserConstructionScript`)