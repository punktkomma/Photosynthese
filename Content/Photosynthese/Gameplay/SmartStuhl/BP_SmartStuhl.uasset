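; BP_SmartStuhl is an interactable chair that the player can sit on and get up from, with Interact toggling on IsUsed.
; Sitting switches player rotation to follow movement, sets a "Chair" motion warp target at the chair's transform and plays the stand-to-sit montage.
; Chair collision is switched off and back on within the same call, without waiting for the montage.
; Standing up stops the current montage and clears IsUsed, without restoring rotation settings.
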(event `/Game/ThirdPerson/Blueprints/BPI_Interact.Interact`
  (params (IsUsed :type Boolean))
  (bind _isused (`self.isUsed`))
  (message `/Game/ThirdPerson/Blueprints/BPI_Interact.Interact` (`GameplayStatics.GetPlayerCharacter` 0) _isused)
  (if _isused
    (`self.StopSitting`)
    (else
      (`self.SittingStart`))))

(event `SittingStart`
  (bind _returnvalue (`GameplayStatics.GetPlayerCharacter` 0))
  (bind (_returnvalue_roll _returnvalue_pitch _returnvalue_yaw) (`KismetMathLibrary.BreakRotator` (`self.K2_GetActorRotation`)))
  (bind _charactermovement (`Character.CharacterMovement` _returnvalue))
  (set `self.isUsed` true)
  (`self.SetActorEnableCollision` false)
  (set `CharacterMovementComponent.bUseControllerDesiredRotation` false _charactermovement)
  (set `CharacterMovementComponent.bOrientRotationToMovement` true _charactermovement)
  (set `Pawn.bUseControllerRotationYaw` false _returnvalue)
  (set `Pawn.bUseControllerRotationRoll` false _returnvalue)
  (`MotionWarpingComponent.AddOrUpdateWarpTargetFromTransform` (`self.GetComponentByClass` _returnvalue "/Script/MotionWarping.MotionWarpingComponent") "Chair" (`KismetMathLibrary.MakeTransform` (`self.K2_GetActorLocation`) (`KismetMathLibrary.MakeRotator` _returnvalue_roll _returnvalue_pitch _returnvalue_yaw)))
  (`Character.PlayAnimMontage` _returnvalue "/Game/Characters/Mannequins/Animations/SitY-StandToSit_Anim_Montage.SitY-StandToSit_Anim_Montage" 1.0 "None")
  (`self.SetActorEnableCollision` true))

(event `StopSitting`
  (bind _returnvalue (`GameplayStatics.GetPlayerCharacter` 0))
  (`Character.StopAnimMontage` _returnvalue (`Character.GetCurrentMontage` _returnvalue))
  (set `self.isUsed` false))

(fn `UserConstructionScript`)