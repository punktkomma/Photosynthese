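; Timed spawner that populates the world with BP_AI_SpawnerAll actors, counted as patients, at its own location.
; From BeginPlay, a timer with a random delay calls SpawnAI, which spawns one actor and gives it a random skeletal mesh.
; It then stores the last index of all such actors (count minus one) and re-arms the timer.
; Once that value equals PatientsMax the timer is not re-armed, so spawning stops.
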(event `self.ReceiveBeginPlay`
  (`/Engine/EditorBlueprintResources/StandardMacros.DoOnce` false
    (:`Completed`
      (`self.ResetTimer`))))

(event `ResetTimer`
  (bind _output_get (set `self.RandomTime` (`KismetMathLibrary.RandomFloatInRange` (`self.MinSpawnTime`) (`self.MaxSpawnTime`))))
  (`KismetSystemLibrary.K2_SetTimerDelegate` (delegate `Spawn AI`) _output_get))

(event `Spawn AI`
  (if (not (== (`self.PatientsInWorld`) (`self.PatientsMax`)))
    (bind _returnvalue (`|SpawnActorFromClass` "/Game/Characters/AI/BP_AI_SpawnerAll.BP_AI_SpawnerAll_C" (`KismetMathLibrary.MakeTransform` (`self.K2_GetActorLocation` self)) "AdjustIfPossibleButDontSpawnIfColliding" "MultiplyWithRoot" null null))
    (`SkeletalMeshComponent.SetSkeletalMeshAsset` (`Character.Mesh` _returnvalue) (`KismetArrayLibrary.Array_Random` (`self.Meshes`)))
    ;[1 0.4091 0.8945] Count all Patients in World
    (bind _outactors (`GameplayStatics.GetAllActorsOfClass` "/Game/Characters/AI/BP_AI_SpawnerAll.BP_AI_SpawnerAll_C"))
    (set `self.PatientsInWorld` (`KismetArrayLibrary.Array_LastIndex` _outactors))
    (`self.ResetTimer`)))

(fn `UserConstructionScript`)