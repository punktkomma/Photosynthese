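; BP_Spawn is a spawner actor that keeps spawning BP_AI_Spawner instances at its own location.
; On BeginPlay it starts a timer with a random delay between MinSpawnTime and MaxSpawnTime, then re-rolls that delay after every spawn.
; Spawns ignore collision, and a step to give each one a random skeletal mesh from Meshes is present but disconnected.
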(event `self.ReceiveBeginPlay`
  (`self.ResetTimer`))

(event `ResetTimer`
  (bind _output_get (set `self.RandomTime` (`KismetMathLibrary.RandomFloatInRange` (`self.MinSpawnTime`) (`self.MaxSpawnTime`))))
  (`KismetSystemLibrary.K2_SetTimerDelegate` (delegate `Spawn AI`) _output_get))

(event `Spawn AI`
  (bind _returnvalue (`|SpawnActorFromClass` "/Game/Characters/AI/BP_AI_Spawner.BP_AI_Spawner_C" (`KismetMathLibrary.MakeTransform` (`self.K2_GetActorLocation` self)) "AlwaysSpawn" "MultiplyWithRoot" null null))
  (`self.ResetTimer`))

(fn `UserConstructionScript`)