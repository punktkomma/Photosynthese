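; Smart object behavior for a chair that makes a triggered character play a sitting-spot animation.
; On trigger it disables the chair's collision and sets a "Chair" motion warp target at the chair's transform so the montage aligns to it.
; It plays a random montage from MontageToPlay on the avatar's mesh, then on completion or interruption ends the behavior and restores collision.
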(event `self.K2_OnTriggeredCharacter`
  (params (Avatar :type "Character Object Reference") (Config :type "GameplayBehaviorConfig Object Reference") (SmartObjectOwner :type "Actor Object Reference"))
  (bind _output_get (set `self.Avatar` Avatar))
  (`Actor.SetActorEnableCollision` SmartObjectOwner false)
  (`MotionWarpingComponent.AddOrUpdateWarpTargetFromTransform` (`Actor.GetComponentByClass` _output_get "/Script/MotionWarping.MotionWarpingComponent") "Chair" (`Actor.GetTransform` SmartObjectOwner))
  (`|PlayMontage` (`Actor.GetComponentByClass` Avatar "/Script/Engine.SkeletalMeshComponent") (`KismetArrayLibrary.Array_Random` (`self.Montage to Play`))
    (:`OnCompleted`
      _)
    (:`OnInterrupted`
      _))
  (`self.K2_EndBehavior` (`self.Avatar`))
  (`Actor.SetActorEnableCollision` SmartObjectOwner true))