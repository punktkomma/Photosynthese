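; BP_AcidPhone is a phone actor that rings at random intervals.
; On BeginPlay it picks a random delay between MinRingTime and MaxRingTime and sets a timer on the Ringing event.
; Ringing plays a quiet, attenuated ring sound at the actor's location, then resets the timer with a new random delay, so the interval varies despite the looping timer.
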(event `self.ReceiveBeginPlay`
  (`self.ResetTimer`))

(event `ResetTimer`
  (bind _output_get (set `self.Random Time` (`KismetMathLibrary.RandomFloatInRange` (`self.Min Ring Time`) (`self.Max Ring Time`))))
  (`KismetSystemLibrary.K2_SetTimerDelegate` (delegate `Ringing`) _output_get true))

(event `Ringing`
  (`GameplayStatics.PlaySoundAtLocation` "/Game/Photosynthese/Gameplay/AudioPraxis/Files/APr_PhoneRing.APr_PhoneRing" (`self.K2_GetActorLocation` self) (`self.K2_GetActorRotation` self) 0.3 1.0 0.0 "/Game/Photosynthese/Audio/Praxis/AttentSpat/SA_Small.SA_Small" null null null)
  (`self.ResetTimer`))

(fn `UserConstructionScript`)