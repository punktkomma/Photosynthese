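; BP_Laterne is a lantern actor that animates blue and red emissive materials on its mesh in response to a KickTrigger event.
; BeginPlay creates dynamic material instances from LaterneBlue and LaterneRed on two slots of the StaticMeshComponent.
; Each KickTrigger call alternates via a FlipFlop between two timelines, each driving the "Int" scalar parameter of the blue or red material, starting with blue.
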(event `self.ReceiveBeginPlay`
  (`|ExecutionSequence`
    (:`then_0`
      (bind _returnvalue (`PrimitiveComponent.CreateDynamicMaterialInstance` (`self.StaticMeshComponent`) 3 "/Game/Level1/Models/LaternenEmissionRB/LaterneBlue.LaterneBlue" "None"))
      (set `self.DynamicMatBlue` _returnvalue))
    (:`then_1`
      (bind _returnvalue_2 (`PrimitiveComponent.CreateDynamicMaterialInstance` (`self.StaticMeshComponent`) 1 "/Game/Level1/Models/LaternenEmissionRB/LaterneRed.LaterneRed" "None"))
      (set `self.DynamicMatRed` _returnvalue_2))))

(event `/Game/Level1/Gameplay/Interface/AudioReactive.KickTrigger`
  (`/Engine/EditorBlueprintResources/StandardMacros.FlipFlop`
    (:`A`
      (bind (_direction _newtrack_0) (`Timeline|Timeline` :!via `PlayFromStart`)
        (:`Update`
          (`MaterialInstanceDynamic.SetScalarParameterValue` (`self.DynamicMatBlue`) "Int" _newtrack_0))))
    (:`B`
      (bind (_direction_2 _newtrack_0_2) (`Timeline|Timeline_0` :!via `PlayFromStart`)
        (:`Update`
          (`MaterialInstanceDynamic.SetScalarParameterValue` (`self.DynamicMatRed`) "Int" _newtrack_0_2))))))

(fn `UserConstructionScript`)