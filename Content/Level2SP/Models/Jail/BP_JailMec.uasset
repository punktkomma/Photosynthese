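; BP_JailMec is a jail that opens when its box trigger is overlapped and releases a second character.
; The first overlap, gated by DoOnce, plays a timeline that swings the door open on yaw.
; The skeletal mesh then plays a joyful jump and, after a short delay, spawns BP_SPSecondChar at its location with a yaw offset.
; The mesh's visibility then toggles, swapping it for the spawned actor.
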(event `self.Box.OnComponentBeginOverlap`
  (params (OverlappedComponent :type "PrimitiveComponent Object Reference") (OtherActor :type "Actor Object Reference") (OtherComp :type "PrimitiveComponent Object Reference") (OtherBodyIndex :type Integer) (bFromSweep :type Boolean) (SweepResult :type "HitResult Structure (by ref)"))
  (bind _skeletalmesh (`self.SkeletalMesh`))
  (bind (_returnvalue_roll _returnvalue_pitch _returnvalue_yaw) (`KismetMathLibrary.BreakRotator` (`SceneComponent.K2_GetComponentRotation` _skeletalmesh)))
  (`/Engine/EditorBlueprintResources/StandardMacros.DoOnce` false
    (:`Completed`
      (bind (_direction _newtrack_2) (`Timeline|Timeline`)
        (:`Update`
          (`SceneComponent.K2_SetRelativeRotation` (`self.Door`) (`KismetMathLibrary.MakeRotator` 0.0 0.0 _newtrack_2) false false))
        (:`Finished`
          (`SkeletalMeshComponent.PlayAnimation` (`self.SkeletalMesh`) "/Game/Photosynthese/Human/Sabine/Animations/Adds/Y2S-Y-JoyfulJump.Y2S-Y-JoyfulJump" false)
          (`KismetSystemLibrary.Delay` 1.5)
          (`|SpawnActorFromClass` "/Game/Level2SP/SecondPerson/SecondCharAi/BP_SPSecondChar.BP_SPSecondChar_C" (`KismetMathLibrary.MakeTransform` (`SceneComponent.K2_GetComponentLocation` _skeletalmesh) (`KismetMathLibrary.MakeRotator` _returnvalue_roll _returnvalue_pitch (+ _returnvalue_yaw 81.509207))) "AlwaysSpawn" "OverrideRootScale" null null)
          (`SceneComponent.ToggleVisibility` _skeletalmesh false))))))

(fn `UserConstructionScript`)