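; Jail cell in Level 2 that opens once when something first overlaps its box and releases three captives.
; A timeline swings the door open in yaw, then the three skeletal meshes play a joyful jump animation.
; After a short delay, each mesh spawns a BP_SPSecondChar at its position with a yaw offset and hides, and the jail and door lose collision.
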(event `self.ReceiveBeginPlay`
  (`PrimitiveComponent.SetCollisionEnabled` (`self.StaticMesh`) "QueryOnly"))

(event `self.Box.OnComponentBeginOverlap`
  (params (OverlappedComponent :type "PrimitiveComponent Object Reference") (OtherActor :type "Actor Object Reference") (OtherComp :type "PrimitiveComponent Object Reference") (OtherBodyIndex :type Integer) (bFromSweep :type Boolean) (SweepResult :type "HitResult Structure (by ref)"))
  (bind _skeletalmesh2 (`self.SkeletalMesh2`))
  (bind _skeletalmesh (`self.SkeletalMesh`))
  (bind _skeletalmesh1 (`self.SkeletalMesh1`))
  (bind (_returnvalue_roll _returnvalue_pitch _returnvalue_yaw) (`KismetMathLibrary.BreakRotator` (`SceneComponent.K2_GetComponentRotation` _skeletalmesh)))
  (bind (_returnvalue_roll_2 _returnvalue_pitch_2 _returnvalue_yaw_2) (`KismetMathLibrary.BreakRotator` (`SceneComponent.K2_GetComponentRotation` _skeletalmesh2)))
  (bind (_returnvalue_roll_3 _returnvalue_pitch_3 _returnvalue_yaw_3) (`KismetMathLibrary.BreakRotator` (`SceneComponent.K2_GetComponentRotation` _skeletalmesh1)))
  (`/Engine/EditorBlueprintResources/StandardMacros.DoOnce` false
    (:`Completed`
      (bind (_direction _newtrack_2) (`Timeline|Timeline`)
        (:`Update`
          (`SceneComponent.K2_SetRelativeRotation` (`self.Door`) (`KismetMathLibrary.MakeRotator` 0.0 0.0 _newtrack_2) false false))
        (:`Finished`
          (`SkeletalMeshComponent.PlayAnimation` (`self.SkeletalMesh`) "/Game/Photosynthese/Human/Sabine/Animations/Adds/Y2S-Y-JoyfulJump.Y2S-Y-JoyfulJump" false)
          (`SkeletalMeshComponent.PlayAnimation` (`self.SkeletalMesh1`) "/Game/Photosynthese/Human/Sabine/Animations/Adds/Y2S-Y-JoyfulJump.Y2S-Y-JoyfulJump" false)
          (`SkeletalMeshComponent.PlayAnimation` (`self.SkeletalMesh2`) "/Game/Photosynthese/Human/Sabine/Animations/Adds/Y2S-Y-JoyfulJump.Y2S-Y-JoyfulJump" false)
          (`KismetSystemLibrary.Delay` 1.5)
          (`|ExecutionSequence`
            (:`then_0`
              (`|SpawnActorFromClass` "/Game/Level2SP/SecondPerson/SecondCharAi/BP_SPSecondChar.BP_SPSecondChar_C" (`KismetMathLibrary.MakeTransform` (`SceneComponent.K2_GetComponentLocation` _skeletalmesh) (`KismetMathLibrary.MakeRotator` _returnvalue_roll _returnvalue_pitch (+ _returnvalue_yaw 81.509207))) "AdjustIfPossibleButAlwaysSpawn" "OverrideRootScale" null null)
              (`SceneComponent.ToggleVisibility` _skeletalmesh false)
              (`PrimitiveComponent.SetCollisionEnabled` (`self.StaticMesh`) "NoCollision")
              (`PrimitiveComponent.SetCollisionEnabled` (`self.Door`) "NoCollision"))
            (:`then_1`
              (`|SpawnActorFromClass` "/Game/Level2SP/SecondPerson/SecondCharAi/BP_SPSecondChar.BP_SPSecondChar_C" (`KismetMathLibrary.MakeTransform` (`SceneComponent.K2_GetComponentLocation` _skeletalmesh1) (`KismetMathLibrary.MakeRotator` _returnvalue_roll_3 _returnvalue_pitch_3 (+ _returnvalue_yaw_3 81.509207))) "AdjustIfPossibleButAlwaysSpawn" "OverrideRootScale" null null)
              (`SceneComponent.ToggleVisibility` _skeletalmesh1 false))
            (:`then_2`
              (`|SpawnActorFromClass` "/Game/Level2SP/SecondPerson/SecondCharAi/BP_SPSecondChar.BP_SPSecondChar_C" (`KismetMathLibrary.MakeTransform` (`SceneComponent.K2_GetComponentLocation` _skeletalmesh2) (`KismetMathLibrary.MakeRotator` _returnvalue_roll_2 _returnvalue_pitch_2 (+ _returnvalue_yaw_2 81.509207))) "AdjustIfPossibleButAlwaysSpawn" "OverrideRootScale" null null)
              (`SceneComponent.ToggleVisibility` _skeletalmesh2 false))))))))

(fn `UserConstructionScript`)