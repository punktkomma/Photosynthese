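; BP_Jury is a jury member actor for Level4Cat that sits down when triggered.
; The construction script gives its skeletal mesh a random asset from the Patients array.
; The JuryTrigger event plays the sit-down animation once, without looping.
; An unconnected Timeline that would shrink the mesh's Z scale and print a debug message never runs.
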(event `/Game/Level4Cat/Audio/BPI_JuryAudio.JuryTrigger`
  (`SkeletalMeshComponent.PlayAnimation` (`self.SkeletalMesh`) "/Game/Photosynthese/Human/Sabine/Animations/Adds/Hum-Sabine_JurySitdown.Hum-Sabine_JurySitdown" false))

(fn `UserConstructionScript`
  (`SkeletalMeshComponent.SetSkeletalMeshAsset` (`self.SkeletalMesh`) (`KismetArrayLibrary.Array_Random` (`self.Patients`))))