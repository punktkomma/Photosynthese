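; BP_CatLawyer is a cat lawyer character that walks in a circle while rising to "heaven", then disappears.
; Its AudioReactive event stores the current location, waits briefly, then starts a looping walk-in-circle animation on the skeletal mesh.
; A Timeline lerps the actor's relative location from that stored world position to HeavenLocation, then destroys the actor when finished.
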(event `/Game/Level4Cat/Audio/BPI_CatAudio.AudioReactive`
  (set `self.EarthLocation` (`self.K2_GetActorLocation`))
  (`KismetSystemLibrary.Delay` 3.0)
  (`SkeletalMeshComponent.PlayAnimation` (`self.SkeletalMesh`) "/Game/Level4Cat/Hum/CatLawyer/A-CatLawyer-Walk_In_Circle.A-CatLawyer-Walk_In_Circle" true)
  (bind (_direction _newtrack_0) (`Timeline|Timeline`)
    (:`Update`
      (`self.K2_SetActorRelativeLocation` (`KismetMathLibrary.VLerp` (`self.EarthLocation`) (`self.HeavenLocation`) _newtrack_0)))
    (:`Finished`
      (`self.K2_DestroyActor`))))

(fn `UserConstructionScript`)