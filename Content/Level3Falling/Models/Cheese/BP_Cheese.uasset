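; BP_Cheese is a cheese actor in the falling level that glows, then animates its scale and position when triggered.
; BeginPlay gives the mesh a dynamic material instance.
; The CheeseGlow event starts a timeline that drives Emissive to a high intensity and, in parallel, starts a five-second delay.
; After the delay, it disables collision and a second timeline's single track drives both actor scale and a cumulative vertical mesh offset.
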(event `self.ReceiveBeginPlay`
  (bind _returnvalue (`PrimitiveComponent.CreateDynamicMaterialInstance` (`self.StaticMeshComponent`) 0 "/Game/Level3Falling/Models/Cheese/M-Cheese_Inst.M-Cheese_Inst" "None"))
  (bind _output_get (set `self.CheeseMaterial` _returnvalue))
  (`PrimitiveComponent.SetMaterial` (`self.StaticMeshComponent`) 0 _output_get))

(event `CheeseGlow`
  (`|ExecutionSequence`
    (:`then_0`
      (bind (_direction _newtrack_0) (`Timeline|GlowHard`)
        (:`Update`
          (`MeshComponent.SetScalarParameterValueOnMaterials` (`self.StaticMeshComponent`) "Emissive" (`KismetMathLibrary.Lerp` 0.0 1000.0 _newtrack_0)))))
    (:`then_1`
      (`KismetSystemLibrary.Delay` 5.0)
      (`PrimitiveComponent.SetCollisionEnabled` (`self.StaticMeshComponent`) "NoCollision")
      (bind (_direction_2 _newtrack_0_2) (`Timeline|Timeline`)
        (:`Update`
          (`self.SetActorRelativeScale3D` (`KismetMathLibrary.MakeVector` _newtrack_0_2 _newtrack_0_2 _newtrack_0_2))
          (`SceneComponent.K2_AddRelativeLocation` (`self.StaticMeshComponent`) (`KismetMathLibrary.MakeVector` 0.0 0.0 (* _newtrack_0_2 10.0)) false false))))))

(fn `UserConstructionScript`)