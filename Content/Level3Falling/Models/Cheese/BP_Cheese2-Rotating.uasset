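; Rotating cheese actor for the falling level that glows and then animates its scale when its CheeseGlow event fires.
; BeginPlay gives the static mesh a dynamic material instance and copies the RotationRate variable to the RotatingMovement component.
; CheeseGlow runs a timeline that drives the Emissive parameter, then disables collision and starts a second timeline that drives the actor's relative scale.
; Nothing in this graph calls CheeseGlow.
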(event `self.ReceiveBeginPlay`
  (bind _returnvalue (`PrimitiveComponent.CreateDynamicMaterialInstance` (`self.StaticMesh`) 0 "/Game/Level3Falling/Models/Cheese/M-Cheese_Inst.M-Cheese_Inst" "None"))
  (bind _output_get (set `self.CheeseMaterial` _returnvalue))
  (`PrimitiveComponent.SetMaterial` (`self.StaticMesh`) 0 _output_get)
  (set `RotatingMovementComponent.RotationRate` (`self.Rotation Rate`) (`self.RotatingMovement`)))

(event `CheeseGlow`
  (bind (_direction _newtrack_0) (`Timeline|GlowHard`)
    (:`Update`
      (`MeshComponent.SetScalarParameterValueOnMaterials` (`self.StaticMesh`) "Emissive" (`KismetMathLibrary.Lerp` 0.0 1000.0 _newtrack_0)))
    (:`Finished`
      (`PrimitiveComponent.SetCollisionEnabled` (`self.StaticMesh`) "NoCollision")
      (bind (_direction_2 _newtrack_0_2) (`Timeline|Timeline`)
        (:`Update`
          (`self.SetActorRelativeScale3D` (`KismetMathLibrary.MakeVector` _newtrack_0_2 _newtrack_0_2 _newtrack_0_2)))))))

(fn `UserConstructionScript`)